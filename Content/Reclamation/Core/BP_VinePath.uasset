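; Spline-and-instanced-mesh vine path whose current element decides how it interacts with boulders.
; Element changes set PhysicsBody collision: Electric and None overlap, destroying the vine when a boulder enters (Electric electrifies it first), while Wind and Corruption block.
; In Wind, Tick applies a distance-limited force pushing boulders away from their closest spline point, using a periodically refreshed boulder list and drawing debug output.
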(event `ChangeElement`
  (`PrimitiveComponent.SetCollisionResponseToChannel` (`self.InstancedStaticMesh`) "ECC_PhysicsBody" (select `/Game/Reclamation/Core/E_Element` (`self.Element`) :`NewEnumerator0` "ECR_Overlap" :`NewEnumerator1` "ECR_Block" :`NewEnumerator2` "ECR_Block" :`NewEnumerator3` "ECR_Overlap" :!type "ECollisionResponse Enum")))

(event `self.ReceiveTick`
  (params (DeltaSeconds :type "Float (single-precision)"))
  (bind _bouldersonlevel (`self.BouldersOnLevel`))
  (if (`|EnumEquality` (`self.Element`) "NewEnumerator1")
    (`|ExecutionSequence`
      (:`then_0`
        (`/Engine/EditorBlueprintResources/StandardMacros.DoOnce` false :!label _label
          (:`Completed`
            (bind _outactors (`GameplayStatics.GetAllActorsOfClass` "/Game/Reclamation/Core/BP_Boulder.BP_Boulder_C"))
            (set `self.BouldersOnLevel` _outactors)
            (`KismetSystemLibrary.Delay` 0.5)
            (goto _label :!via `Reset`))))
      (:`then_1`
        (if (`KismetArrayLibrary.Array_IsNotEmpty` _bouldersonlevel)
          (for _array_element _bouldersonlevel
            (bind _sphere (`/Game/Reclamation/Core/BP_Boulder.Sphere` _array_element))
            (bind _returnvalue (`SceneComponent.K2_GetComponentLocation` _sphere))
            (bind _returnvalue_2 (`SplineComponent.FindLocationClosestToWorldLocation` (`self.Spline`) _returnvalue "World"))
            (`KismetSystemLibrary.DrawDebugArrow` _returnvalue_2 _returnvalue 100.0)
            (bind _returnvalue_3 (- _returnvalue _returnvalue_2))
            (bind _returnvalue_4 (* (`KismetMathLibrary.FMax` (- 900.0 (`KismetMathLibrary.VSize` _returnvalue_3))) 0.01))
            (`KismetSystemLibrary.PrintString` (`KismetStringLibrary.Conv_DoubleToString` _returnvalue_4))
            (`PrimitiveComponent.AddForce` _sphere (* _returnvalue_3 _returnvalue_4) "None" true)))))))

(event `ElementInfusion`
  (`self.Element infusion`))

(event `self.InstancedStaticMesh.OnComponentBeginOverlap`
  (params (OverlappedComponent :type "PrimitiveComponent Object Reference") (OtherActor :type "Actor Object Reference") (OtherComp :type "PrimitiveComponent Object Reference") (OtherBodyIndex :type Integer) (bFromSweep :type Boolean) (SweepResult :type "HitResult Structure (by ref)"))
  (bind _asbp_boulder (cast `/Game/Reclamation/Core/BP_Boulder` OtherActor))
  (set `self.Boulder Hit` _asbp_boulder)
  (switch `/Game/Reclamation/Core/E_Element` (`self.Element`)
    (:`NewEnumerator0`
      (`/Game/Reclamation/Core/BP_Boulder.Electrify Boulder` (`self.Boulder Hit`))
      (`self.K2_DestroyActor`))
    (:`NewEnumerator3`
      (`self.K2_DestroyActor`))))

(fn `UserConstructionScript`)