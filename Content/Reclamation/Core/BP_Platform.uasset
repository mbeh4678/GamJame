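; BP_Platform is a moving platform that carries a cube back and forth along a spline.
; Tick advances a timer scaled by Duration and folds it into a ping-pong alpha, so each one-way trip takes Duration seconds.
; That alpha is eased by a selectable interpolation type into a distance along the spline, which sets the cube's world location.
; The cube either follows the spline's rotation or keeps the rotation cached at BeginPlay.
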(event `self.ReceiveBeginPlay`
  (set `self.Starting Rotation` (`SceneComponent.K2_GetComponentRotation` (`self.Cube`))))

(event `self.ReceiveTick`
  (params (DeltaSeconds :type "Float (single-precision)"))
  (bind _spline (`self.Spline`))
  (bind _returnvalue (mod (`self.TimerTracker`) 1.0))
  (bind _output_get (set `self.TimerTracker` (+ (* DeltaSeconds (/ 1.0 (`self.Duration`))) (`self.TimerTracker`))))
  (bind (_returnvalue_location _returnvalue_rotation) (`KismetMathLibrary.BreakTransform` (`SplineComponent.GetTransformAtDistanceAlongSpline` _spline (`|EaseFunction` (`self.Interpolation Type`) (select `bool` (< (mod _output_get 2.0) 1.0) :`false` (- 1.0 _returnvalue) :`true` _returnvalue) 0.0 (`SplineComponent.GetSplineLength` _spline)) "World" false)))
  (`SceneComponent.K2_SetWorldLocationAndRotation` (`self.Cube`) _returnvalue_location (select `bool` (`self.FollowSplineRotation`) :`false` (`self.Starting Rotation`) :`true` _returnvalue_rotation) false false))

(fn `UserConstructionScript`)