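; BP_Sconce is an elemental sconce that passes its Element (Electric, Wind, Corruption or None) to vine paths it touches.
; The construction script colors Sphere with the element's material, and BeginPlay plays the matching sound there.
; When Sphere1 begins overlapping a BP_VinePath, it sets that path's Element and instanced-mesh material.
; Tick uses a FlipFlop to nudge Sphere1 up and down with sweep on alternate frames.
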(event `Select Sound`
  (`GameplayStatics.PlaySoundAtLocation` (select `/Game/Reclamation/Core/E_Element` (`self.Element`) :`NewEnumerator0` "/Game/AdvancedLocomotionV4/Sounds/Electricity.Electricity" :`NewEnumerator1` "/Game/AdvancedLocomotionV4/Sounds/Wind.Wind" :`NewEnumerator2` "/Game/AdvancedLocomotionV4/Sounds/Goopy_-_Goopy.Goopy_-_Goopy" :!type "SoundBase Object Reference") (`SceneComponent.K2_GetComponentLocation` (`self.Sphere`)) (struct) 1.0 1.0 0.0 null null null null))

(event `self.ReceiveBeginPlay`
  (`self.Select Sound`))

(event `self.ReceiveTick`
  (params (DeltaSeconds :type "Float (single-precision)"))
  (bind _sphere1 (`self.Sphere1`))
  (`/Engine/EditorBlueprintResources/StandardMacros.FlipFlop`
    (:`A`
      (`SceneComponent.K2_AddLocalOffset` _sphere1 (0.0 0.0 0.1) true false))
    (:`B`
      (`SceneComponent.K2_AddLocalOffset` _sphere1 (0.0 0.0 -0.1) true false))))

(event `self.Sphere1.OnComponentBeginOverlap`
  (params (OverlappedComponent :type "PrimitiveComponent Object Reference") (OtherActor :type "Actor Object Reference") (OtherComp :type "PrimitiveComponent Object Reference") (OtherBodyIndex :type Integer) (bFromSweep :type Boolean) (SweepResult :type "HitResult Structure (by ref)"))
  (bind _element (`self.Element`))
  (bind _asbp_vine_path (cast `/Game/Reclamation/Core/BP_VinePath` OtherActor))
  (set `/Game/Reclamation/Core/BP_VinePath.Element` _element _asbp_vine_path)
  (`PrimitiveComponent.SetMaterial` (`/Game/Reclamation/Core/BP_VinePath.InstancedStaticMesh` _asbp_vine_path) 0 (select `/Game/Reclamation/Core/E_Element` _element :`NewEnumerator0` "/Game/Reclamation/Core/MI_Electrified.MI_Electrified" :`NewEnumerator1` "/Game/Reclamation/Core/MI_Wind.MI_Wind" :`NewEnumerator2` "/Game/Reclamation/Core/MI_Corrupted.MI_Corrupted" :`NewEnumerator3` "/Game/Reclamation/Core/M_Basic.M_Basic" :!type "MaterialInterface Object Reference")))

(fn `UserConstructionScript`
  (`PrimitiveComponent.SetMaterial` (`self.Sphere`) 0 (select `/Game/Reclamation/Core/E_Element` (`self.Element`) :`NewEnumerator0` "/Game/Reclamation/Core/MI_Electrified.MI_Electrified" :`NewEnumerator1` "/Game/Reclamation/Core/MI_Wind.MI_Wind" :`NewEnumerator2` "/Game/Reclamation/Core/MI_Corrupted.MI_Corrupted" :`NewEnumerator3` "/Game/Reclamation/Core/M_Basic.M_Basic" :!type "MaterialInterface Object Reference")))