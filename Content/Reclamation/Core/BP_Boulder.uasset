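; BP_Boulder is a boulder actor with an element state that can switch to an electrified look.
; ElectrifyBoulder sets the Sphere's electrified material and element, and Tick reapplies it every frame while that element is active.
; A Sphere hit against another BP_Boulder electrifies that boulder, without checking the element of the one reporting the hit.
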(event `self.ReceiveTick`
  (params (DeltaSeconds :type "Float (single-precision)"))
  (if (`|EnumEquality` (`self.Element`) "NewEnumerator0")
    (`self.Electrify Boulder`)))

(event `Electrify Boulder`
  (`PrimitiveComponent.SetMaterial` (`self.Sphere`) 0 "/Game/Reclamation/Core/MI_Electrified.MI_Electrified")
  (set `self.Element` "NewEnumerator0"))

(event `self.Sphere.OnComponentHit`
  (params (HitComponent :type "PrimitiveComponent Object Reference") (OtherActor :type "Actor Object Reference") (OtherComp :type "PrimitiveComponent Object Reference") (NormalImpulse :type "Vector Structure") (Hit :type "HitResult Structure (by ref)"))
  (bind _asbp_boulder (cast `/Game/Reclamation/Core/BP_Boulder` OtherActor))
  (`self.Electrify Boulder` _asbp_boulder))

(fn `UserConstructionScript`)