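; BP_Door is a door that opens when a BP_VinePath or BP_Boulder of its DesiredElement comes near its front.
; Tick runs a sphere overlap ahead of the door, with an optional debug draw, and checks the Element of each hit actor.
; A match, or a call to the OpenDoor event, raises the Cube via MoveComponentTo, with no closing logic.
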(event `self.ReceiveTick`
  (params (DeltaSeconds :type "Float (single-precision)"))
  (bind _defaultsceneroot (`self.DefaultSceneRoot`))
  (bind _returnvalue (+ (`SceneComponent.K2_GetComponentLocation` _defaultsceneroot) (* (`SceneComponent.GetForwardVector` _defaultsceneroot) 150.0)))
  (if (`self.Debug sphere`)
    (`KismetSystemLibrary.DrawDebugSphere` _returnvalue 100.0 12 (struct :`R` 1.0 :`A` 1.0)))
  (bind (_outactors _returnvalue_2) (`KismetSystemLibrary.SphereOverlapActors` _returnvalue 100.0 (`|MakeArray` "ObjectTypeQuery7" "ObjectTypeQuery4" :!type "EObjectTypeQuery Enum")))
  (if _returnvalue_2
    (for _array_element _outactors
      (bind _asbp_vine_path (cast `/Game/Reclamation/Core/BP_VinePath` _array_element)
        (:`then`
          (if (`|EnumEquality` (`/Game/Reclamation/Core/BP_VinePath.Element` _asbp_vine_path) (`self.Desired Element`))
            (`KismetSystemLibrary.MoveComponentTo` (`self.Cube`) (0.0 0.0 400.0) (struct) false false 2.0 :!label _label)))
        (:`CastFailed`
          (bind _asbp_boulder (cast `/Game/Reclamation/Core/BP_Boulder` _array_element))
          (if (`|EnumEquality` (`/Game/Reclamation/Core/BP_Boulder.Element` _asbp_boulder) (`self.Desired Element`))
            (goto _label)))))))

(event `Open Door`
  (goto _label))

(fn `UserConstructionScript`)